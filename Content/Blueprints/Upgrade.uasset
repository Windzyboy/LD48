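; Upgrade is a collectible pickup actor that fires once, either on player overlap when not set to manual pickup or through its Trigger event.
; Collection plays a sound, stops the sparkles and runs a timeline that spins and scales the Upgrade component while blending the Sprite between player and actor positions.
; When the timeline finishes, GiveUpgrade checks for Player_Char and destroys the actor, granting nothing itself.
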(event Custom|GiveUpgrade
  (Utilities|Casting|CastToPlayer_Char (Game|Player|GetPlayerPawn 0))
  (Actor|DestroyActor))

(event Custom|Trigger
  (bind _upgrade (Variables|Default|GetUpgrade))
  (if (not (Variables|Default|GetbHasBeenCollected?))
    (Variables|Default|SetbHasBeenCollected? true)
    (Audio|PlaySound2D "/Game/Sounds/ug.ug" 1.0 1.0 0.0 0 0)
    (Components|Activation|Deactivate (Variables|Default|GetItemSparkles))
    (bind (_direction _rotation _scale _toplayer) (Timeline|Timeline_0 PlayFromStart)
      (:Update
        (Transformation|SetRelativeTransform _upgrade (Math|Transform|MakeTransform (Variables|/Script/Engine.SceneComponent|GetRelativeLocation _upgrade) (Math|Rotator|Lerp(Rotator) "360.000000,0.000000, 0" "0, 0, 0" _rotation) (Math|Conversions|ToVector(Float) _scale)) false false)
        (Transformation|SetWorldLocationAndRotation (Variables|Default|GetSprite) (Math|Vector|Lerp(Vector) (Transformation|GetActorLocation (Game|Player|GetPlayerPawn 0)) (Transformation|GetActorLocation) _toplayer) "0, 0, 0" false false))
      (:Finished
        (CallFunction|GiveUpgrade)))))

(event Collision|EventActorBeginOverlap
  (params (OtherActor :type Actor%20Object%20Reference))
  (bind _upgrade (Variables|Default|GetUpgrade))
  (if (not (Variables|Default|GetbIsManualPickup?))
    (if (== OtherActor (Game|Player|GetPlayerPawn 0))
      (if (not (Variables|Default|GetbHasBeenCollected?))
        (Variables|Default|SetbHasBeenCollected? true)
        (Audio|PlaySound2D "/Game/Sounds/ug.ug" 1.0 1.0 0.0 0 0)
        (Components|Activation|Deactivate (Variables|Default|GetItemSparkles))
        (bind (_direction _rotation _scale _toplayer) (Timeline|Timeline_0 PlayFromStart)
          (:Update
            (Transformation|SetRelativeTransform _upgrade (Math|Transform|MakeTransform (Variables|/Script/Engine.SceneComponent|GetRelativeLocation _upgrade) (Math|Rotator|Lerp(Rotator) "360.000000,0.000000, 0" "0, 0, 0" _rotation) (Math|Conversions|ToVector(Float) _scale)) false false)
            (Transformation|SetWorldLocationAndRotation (Variables|Default|GetSprite) (Math|Vector|Lerp(Vector) (Transformation|GetActorLocation (Game|Player|GetPlayerPawn 0)) (Transformation|GetActorLocation) _toplayer) "0, 0, 0" false false))
          (:Finished
            (CallFunction|GiveUpgrade)))))))

(fn ConstructionScript)