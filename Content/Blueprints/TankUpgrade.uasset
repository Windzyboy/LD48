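; TankUpgrade is an actor that upgrades the player character's oxygen tank and then destroys itself.
; GiveUpgrade casts player pawn 0 to Player_Char and keeps the larger of the player's TankCapacity and its own, so capacity never drops.
; It records the oxygen fill ratio first and rescales Oxygen to the resulting capacity, preserving the tank's percentage.
; The actor is destroyed even when the cast fails.
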(event EventGiveUpgrade
  (bind _asplayer_char (Utilities|Casting|CastToPlayer_Char (Game|Player|GetPlayerPawn 0))
    (:then
      (Variables|Default|SetAs%20Player%20Char _asplayer_char)
      (Variables|Default|SetCurrentOxygenRatio (/ (Variables|/Game/Player_Char.Player_Char_C|GetOxygen _asplayer_char) (Variables|/Game/Player_Char.Player_Char_C|GetTankCapacity _asplayer_char)))
      (Variables|/Game/Player_Char.Player_Char_C|SetTankCapacity (Variables|Default|GetAs%20Player%20Char) (select (> (Variables|/Game/Player_Char.Player_Char_C|GetTankCapacity _asplayer_char) (Variables|Default|GetTankCapacity)) (Variables|/Game/Player_Char.Player_Char_C|GetTankCapacity _asplayer_char) (Variables|Default|GetTankCapacity)))
      (Variables|/Game/Player_Char.Player_Char_C|SetOxygen (Variables|Default|GetAs%20Player%20Char) (* (Variables|Default|GetCurrentOxygenRatio) (Variables|/Game/Player_Char.Player_Char_C|GetTankCapacity (Variables|Default|GetAs%20Player%20Char))))
      (Actor|DestroyActor))
    (:CastFailed
      (Actor|DestroyActor))))

(fn ConstructionScript
  (|CallParentFunction))