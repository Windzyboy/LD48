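; UsableTriggerBase is a usable trigger that animates a sprite indicator when the player is in range and it is not being used.
; Tick polls for overlapping Player_Char actors and plays a timeline that uniformly scales the PaperSprite, reversing it otherwise.
; The construction script places the sprite at a fixed offset above the Box extent, so it follows the trigger's size.
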(event EventTick
  (params (DeltaSeconds :type Float%20%28single-precision%29))
  (if (and (Utilities|Array|IsValidIndex (Collision|GetOverlappingActors "/Game/Player_Char.Player_Char_C" :!class /Script/Engine.Actor)) (not (Variables|Default|GetbIsBeingUsed?)))
    (bind _newtrack_0 (Timeline|Timeline_0 Play)
      (:Update
        (Transformation|SetRelativeScale3D (Variables|Default|GetPaperSprite) (Math|Vector|MakeVector _newtrack_0 _newtrack_0 _newtrack_0))))
    (else
      (Timeline|Timeline_0 Reverse))))

(fn ConstructionScript
  (Transformation|SetRelativeLocation (Variables|Default|GetPaperSprite) (Math|Vector|MakeVector 0.0 0.0 (+ (.z (Variables|/Script/Engine.BoxComponent|GetBoxExtent (Variables|Default|GetBox))) 1e+02)) false false))