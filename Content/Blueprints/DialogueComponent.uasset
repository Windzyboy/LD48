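; Dialogue component that steps through an array of dialogue entries, showing one chat box widget at a time.
; Each NextDialogue call removes the current widget, creates a ChatBox for the indexed entry, advances the index and sets the player character's IsInDialogue flag.
; Past the last entry, it clears the flag and widget, resets the index and sends DialogueComponentFinishedMessage to its owner.
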(event Custom|NextDialogue
  (if (> (Variables|Default|GetDialogueIndex) (Utilities|Array|LastIndex (Variables|Default|GetDialogueStructures)))
    (bind _asplayer_char (Utilities|Casting|CastToPlayer_Char (Game|Player|GetPlayerPawn 0))
      (:then
        (Variables|/Game/Player_Char.Player_Char_C|SetbIsInDialogue? _asplayer_char false))
      (:CastFailed
        _))
    (Utilities|IsValid (Variables|Default|GetCurrentDialogue)
      (:Is%20Valid
        (Widget|RemovefromParent (Variables|Default|GetCurrentDialogue)))
      (:Is%20Not%20Valid
        _))
    (Variables|Default|SetDialogueIndex 0)
    (Class|Interfaces|DialogueComponentFinished(Message) (Components|GetOwner))
    (else
      (Utilities|IsValid (Variables|Default|GetCurrentDialogue)
        (:Is%20Valid
          (Widget|RemovefromParent (Variables|Default|GetCurrentDialogue)))
        (:Is%20Not%20Valid
          _))
      (bind _returnvalue (UserInterface|CreateWidget "/Game/UMG/ChatBox.ChatBox_C" (Game|GetPlayerController 0) (Utilities|Array|Get(acopy) (Variables|Default|GetDialogueStructures) (Variables|Default|GetDialogueIndex))))
      (bind _output_get (Variables|Default|SetCurrentDialogue _returnvalue))
      (UserInterface|Viewport|AddtoViewport _output_get 0)
      (Math|Integer|IncrementInt (Variables|Default|GetDialogueIndex)
        (:%20%20
          (bind _asplayer_char_2 (Utilities|Casting|CastToPlayer_Char (Game|Player|GetPlayerPawn 0)))
          (Variables|/Game/Player_Char.Player_Char_C|SetbIsInDialogue? _asplayer_char_2 true))))))