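; Interactable money pickup that plays its dialogue, then flags the player as having earned money.
; BeginPlay loads the dialogue and caches the player character; Interact advances the dialogue only while the player has not earned money.
; When the dialogue finishes, it deactivates the particles, and a timeline lerps the paper sprite between the actor and the player's live position before destroying the actor.
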(event EventInteract
  (if (not (Variables|/Game/Player_Char.Player_Char_C|GetbHasEarnedMoney? (Variables|Default|GetAs%20Player%20Char)))
    (Default|NextDialogue (Variables|Default|GetDialogueComponent))))

(event EventTick
  (params (DeltaSeconds :type Float%20%28single-precision%29))
  (|CallParentFunction DeltaSeconds))

(event EventBeginPlay
  (Variables|/Game/Blueprints/DialogueComponent.DialogueComponent_C|SetDialogueStructures (Variables|Default|GetDialogueComponent) (Variables|Default|GetDialogue))
  (bind _asplayer_char (Utilities|Casting|CastToPlayer_Char (Game|Player|GetPlayerPawn 0)))
  (Variables|Default|SetAs%20Player%20Char _asplayer_char))

(event EventDialogueComponentFinished
  (Variables|Default|SetbIsBeingUsed? true)
  (Variables|/Game/Player_Char.Player_Char_C|SetbHasEarnedMoney? (Variables|Default|GetAs%20Player%20Char) true)
  (Components|Activation|Deactivate (Variables|Default|GetParticleSystem))
  (bind _toplayer (Timeline|Timeline_1 PlayFromStart)
    (:Update
      (Transformation|SetWorldLocationAndRotation (Variables|Default|GetPaperSprite1) (Math|Vector|Lerp(Vector) (Transformation|GetActorLocation (Game|Player|GetPlayerPawn 0)) (Transformation|GetActorLocation) _toplayer) "0, 0, 0" false false))
    (:Finished
      (Actor|DestroyActor))))

(fn ConstructionScript
  (|CallParentFunction))