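; Info is an interactable Blueprint that plays dialogue through a DialogueComponent.
; BeginPlay copies its Dialogue data into the component and caches the player pawn as Player_Char.
; Each Interact advances to the next dialogue while IsBeingUsed is false.
; When the component reports it has finished, IsBeingUsed is set to true and never cleared here, so later interactions do nothing.
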(event EventInteract
  (if (not (Variables|Default|GetbIsBeingUsed?))
    (Default|NextDialogue (Variables|Default|GetDialogueComponent))))

(event EventTick
  (params (DeltaSeconds :type Float%20%28single-precision%29))
  (|CallParentFunction DeltaSeconds))

(event EventBeginPlay
  (Variables|/Game/Blueprints/DialogueComponent.DialogueComponent_C|SetDialogueStructures (Variables|Default|GetDialogueComponent) (Variables|Default|GetDialogue))
  (bind _asplayer_char (Utilities|Casting|CastToPlayer_Char (Game|Player|GetPlayerPawn 0)))
  (Variables|Default|SetAs%20Player%20Char _asplayer_char))

(event EventDialogueComponentFinished
  (Variables|Default|SetbIsBeingUsed? true))

(fn ConstructionScript
  (|CallParentFunction))