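; Usable trigger that teleports the first player's pawn to DestLocation, with a zeroed rotation, when interacted with.
; Interact fades the camera out, waits for the fade, moves the pawn, then fades the view back in.
; An IsBeingUsed flag ignores repeat interactions until a short delay after the teleport clears it.
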(event EventInteract
  (if (not (Variables|Default|GetbIsBeingUsed?))
    (Variables|Default|SetbIsBeingUsed? true)
    (CameraFades|StartCameraFade :self (Game|GetPlayerCameraManager 0) :ToAlpha 1.0 :Duration 0.5 :bHoldWhenFinished true)
    (Utilities|FlowControl|Delay 0.5)
    (Transformation|Teleport (Game|Player|GetPlayerPawn 0) (Variables|Default|GetDest%20Location) "0, 0, 0")
    (CameraFades|StartCameraFade :self (Game|GetPlayerCameraManager 0) :FromAlpha 1.0 :Duration 0.5 :bHoldWhenFinished true)
    (Utilities|FlowControl|Delay 1.0)
    (Variables|Default|SetbIsBeingUsed? false)))

(event EventTick
  (params (DeltaSeconds :type Float%20%28single-precision%29))
  (|CallParentFunction DeltaSeconds))

(fn ConstructionScript
  (|CallParentFunction))